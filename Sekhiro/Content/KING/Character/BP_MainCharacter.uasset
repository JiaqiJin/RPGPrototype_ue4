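; BP_MainCharacter is the player character Blueprint that supplies camera data through BPI interface functions.
; It builds a third-person pivot from the averaged head and root socket locations with the actor's rotation.
; It returns a shoulder-dependent trace socket for third person, a first-person camera socket, and FOV and shoulder settings.
; The event graph and construction script contain no logic.
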(event EventBeginPlay)

(event Collision|EventActorBeginOverlap
  (params (OtherActor :type Actor%20Object%20Reference)))

(event EventTick
  (params (DeltaSeconds :type Float%20%28single-precision%29)))

(fn ConstructionScript)

(fn BPIGet3PPivotTarget
  (bind _mesh (Variables|Character|GetMesh))
  (return (Math|Transform|MakeTransform (Math|Vector|GetVectorArrayAverage (Utilities|Array|MakeArray (Transformation|GetSocketLocation _mesh "head") (Transformation|GetSocketLocation _mesh "root"))) (Transformation|GetActorRotation))))

(fn BPIGet3PTraceParam
  (if (Variables|Default|GetIsRightShoulder)
    (return (Transformation|GetSocketLocation (Variables|Character|GetMesh) "TP_CameraTrace_R") 1e+01 "TraceTypeQuery1")
    (else
      (return (Transformation|GetSocketLocation (Variables|Character|GetMesh) "TP_CameraTrace_L") 1e+01 "TraceTypeQuery1"))))

(fn BPIGetFPCameraTarget
  (return (Transformation|GetSocketLocation (Variables|Character|GetMesh) "FP_Camera")))

(fn BPIGetCameraParameters
  (return (Variables|Default|GetThirdPerson_FOV) (Variables|Default|GetFirstdPerson_FOV) (Variables|Default|GetIsRightShoulder)))