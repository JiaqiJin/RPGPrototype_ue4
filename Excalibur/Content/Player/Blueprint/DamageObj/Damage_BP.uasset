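; Damage object actor that hurts a hero player character on contact.
; When its Collision component begins overlapping a HeroPlayerCharacter, it calls HeroApplyDamage with its Damage value, passing the hero as both damaged actor and damage causer.
; An unconnected Gameplay Ability System path, which would apply HGE_Damage with a Data.Damage set-by-caller magnitude, remains in the graph but never runs.
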(event OnComponentBeginOverlap(Collision)
  (params (OverlappedComponent :type Primitive%20Component%20Object%20Reference) (OtherActor :type Actor%20Object%20Reference) (OtherComp :type Primitive%20Component%20Object%20Reference) (OtherBodyIndex :type Integer) (bFromSweep :type Boolean) (SweepResult :type Hit%20Result%20Structure%20%28by%20ref%29))
  (bind _ashero_player_character (Utilities|Casting|CastToHeroPlayerCharacter OtherActor))
  (bind _output_get (Variables|Default|SetHero%20Character _ashero_player_character))
  (Class|HeroGameplayStatics|HeroApplyDamage _output_get (Variables|Default|GetDamage) 0 _output_get 0 false))

(event EventBeginPlay)

(event Collision|EventActorBeginOverlap
  (params (OtherActor :type Actor%20Object%20Reference)))

(event EventTick
  (params (DeltaSeconds :type Float%20%28single-precision%29)))

(fn ConstructionScript)